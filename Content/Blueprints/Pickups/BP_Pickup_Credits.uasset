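; Credits pickup that adds currency to the game state when picked up.
; It extends a parent pickup class, assigning the coin burst Niagara effect as its pickup system on BeginPlay.
; On pickup it runs the parent logic, casts the game state to MarsMarine_GameState, adds its credit value, then destroys itself.
; If that cast fails, neither the credit award nor the destroy happens.
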(event `self.ReceiveBeginPlay`
  (`parent.ReceiveBeginPlay`)
  (set `self.PickupSystem` "/Game/sA_PickupSet_1/Fx/NiagaraSystems/NS_CoinBurst.NS_CoinBurst"))

(event `/Game/Blueprints/Interfaces/BPI_Pickeable.PickUp`
  (params (InstigatorActor :type "Actor Object Reference"))
  (`parent.PickUp` InstigatorActor)
  (bind _asmars_marine_game_state (cast `/Game/Core/GameStates/MarsMarine_GameState` (`GameplayStatics.GetGameState`)))
  (`/Game/Core/GameStates/MarsMarine_GameState.AddCredits` _asmars_marine_game_state (`self.CreditsGiven`))
  (`self.K2_DestroyActor`))

(fn `UserConstructionScript`
  (`parent.UserConstructionScript`))