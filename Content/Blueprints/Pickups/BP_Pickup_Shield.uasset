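; BP_Pickup_Shield is a pickup that shields the marine who collects it.
; It extends a parent pickup class, setting its PickupSystem to the NS_Shield effect on BeginPlay.
; On PickUp it runs the parent logic, then, only if the instigator is a BP_Marine, calls SetShielded and destroys itself.
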(event `self.ReceiveBeginPlay`
  (`parent.ReceiveBeginPlay`)
  (set `self.PickupSystem` "/Game/sA_PickupSet_1/Fx/NiagaraSystems/NS_Shield.NS_Shield"))

(event `/Game/Blueprints/Interfaces/BPI_Pickeable.PickUp`
  (params (InstigatorActor :type "Actor Object Reference"))
  (`parent.PickUp` InstigatorActor)
  (bind _asbp_marine (cast `/Game/Blueprints/Pawns/BP_Marine` InstigatorActor))
  (`/Game/Blueprints/Pawns/BP_Marine.SetShielded` _asbp_marine)
  (`self.K2_DestroyActor`))

(fn `UserConstructionScript`
  (`parent.UserConstructionScript`))