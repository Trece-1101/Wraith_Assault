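; Health pickup Blueprint, a child of a pickup parent class, that restores health to the marine who picks it up.
; BeginPlay runs the parent logic, then sets the pickup system to the NS_Healing_1 effect.
; PickUp calls the parent, casts the instigator to BP_Marine, adds HealthGiven and destroys the pickup; other actors leave it in place after the parent call.
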(event `self.ReceiveBeginPlay`
  (`parent.ReceiveBeginPlay`)
  (set `self.PickupSystem` "/Game/sA_PickupSet_1/Fx/NiagaraSystems/NS_Healing_1.NS_Healing_1"))

(event `/Game/Blueprints/Interfaces/BPI_Pickeable.PickUp`
  (params (InstigatorActor :type "Actor Object Reference"))
  (`parent.PickUp` InstigatorActor)
  (bind _asbp_marine (cast `/Game/Blueprints/Pawns/BP_Marine` InstigatorActor))
  (`/Game/Blueprints/Pawns/BP_Marine.AddHealth` _asbp_marine (`self.HealthGiven`))
  (`self.K2_DestroyActor`))

(fn `UserConstructionScript`
  (`parent.UserConstructionScript`))