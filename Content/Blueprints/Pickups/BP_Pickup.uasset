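; Pickup actor that expires on its own five seconds after spawning and provides feedback when picked up.
; On BeginPlay it waits, then spawns its particle system, plays the pickup cue at a much lower pitch and destroys itself.
; The PickUp event plays the cue at the instigator and spawns the effect at the pickup, without applying gameplay effects or destroying the actor.
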(event `self.ReceiveBeginPlay`
  (bind _returnvalue (`self.K2_GetActorLocation`))
  (`KismetSystemLibrary.Delay` 5.0)
  (`NiagaraFunctionLibrary.SpawnSystemAtLocation` (`self.PickupSystem`) _returnvalue)
  (`GameplayStatics.PlaySoundAtLocation` "/Game/Sounds/InterfaceAudio/A_Pickup_Cue.A_Pickup_Cue" _returnvalue (struct) 1.0 0.2 0.0 null null null null)
  (`self.K2_DestroyActor`))

(event `/Game/Blueprints/Interfaces/BPI_Pickeable.PickUp`
  (params (InstigatorActor :type "Actor Object Reference"))
  (bind (_returnvalue_x _returnvalue_y _returnvalue_z) (`KismetMathLibrary.BreakVector` (`self.K2_GetActorLocation`)))
  (`GameplayStatics.PlaySoundAtLocation` "/Game/Sounds/InterfaceAudio/A_Pickup_Cue.A_Pickup_Cue" (`self.K2_GetActorLocation` InstigatorActor) (struct) 1.0 1.0 0.0 null null null null)
  (`NiagaraFunctionLibrary.SpawnSystemAtLocation` (`self.PickupSystem`) (`KismetMathLibrary.MakeVector` _returnvalue_x _returnvalue_y _returnvalue_z)))

(fn `UserConstructionScript`)