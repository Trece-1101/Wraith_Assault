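; BP_WraithProjectile is a projectile that travels at a configurable speed and destroys itself after a set lifetime.
; The construction script copies Speed into the initial and maximum speed of its ProjectileMovement.
; On BeginPlay the collider ignores the instigator when moving, then after the lifetime delay a destroy effect spawns at its transform.
; The collider's overlap event is empty, so overlaps trigger no logic here.
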(event `self.ReceiveBeginPlay`
  (`PrimitiveComponent.IgnoreActorWhenMoving` (`self.Collider`) (`self.GetInstigator`) true)
  (`KismetSystemLibrary.Delay` (`self.LifeTIme`))
  (`NiagaraFunctionLibrary.SpawnSystemAtLocation` (`self.DestroyVFX`) (`self.K2_GetActorLocation`) (`self.K2_GetActorRotation`))
  (`self.K2_DestroyActor`))

(event `self.Collider.OnComponentBeginOverlap`
  (params (OverlappedComponent :type "PrimitiveComponent Object Reference") (OtherActor :type "Actor Object Reference") (OtherComp :type "PrimitiveComponent Object Reference") (OtherBodyIndex :type Integer) (bFromSweep :type Boolean) (SweepResult :type "HitResult Structure (by ref)")))

(fn `UserConstructionScript`
  (bind _projectilemovement (`self.ProjectileMovement`))
  (bind _speed (`self.Speed`))
  (`|ExecutionSequence`
    (:`then_0`
      (set `ProjectileMovementComponent.InitialSpeed` _speed _projectilemovement))
    (:`then_1`
      (set `ProjectileMovementComponent.MaxSpeed` _speed _projectilemovement))))