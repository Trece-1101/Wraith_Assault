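; BP_AreaOfEffect is a temporary area-of-effect hazard that deals repeated radial damage around its location.
; On BeginPlay, a looping timer applies full, falloff-free damage within the damage radius at each tick interval.
; A timeline starts alongside it, driving the uniform world scale of the particle system.
; The construction script sets the actor's lifespan from the effect time, so it removes itself when that expires.
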(event `self.ReceiveBeginPlay`
  (`KismetSystemLibrary.K2_SetTimerDelegate` (delegate `TickDamage`) (`self.TickTime`) true)
  (bind (_direction _newtrack_0) (`Timeline|Timeline`)
    (:`Update`
      (`SceneComponent.SetWorldScale3D` (`self.ParticleSystem`) (`KismetMathLibrary.MakeVector` _newtrack_0 _newtrack_0 _newtrack_0)))))

(event `TickDamage`
  (`GameplayStatics.ApplyRadialDamage` :`BaseDamage` (`self.DamageGivenByTick`) :`Origin` (`self.K2_GetActorLocation`) :`DamageRadius` (`self.DamageRadius`) :`DamageCauser` null :`InstigatedByController` null :`bDoFullDamage` true))

(fn `UserConstructionScript`
  (`self.SetLifeSpan` (`self.EffectTime`)))