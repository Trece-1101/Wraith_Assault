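; BP_Fadeable is a debug Blueprint whose Cube can fade and unfade through a dither material.
; BeginPlay creates a dynamic instance of M_Dither and assigns it to the Cube.
; Fade, guarded by IsFaded against repeat calls, and Unfaded, which clears that flag, each play their own timeline to drive the material's Percent parameter.
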(event `self.ReceiveBeginPlay`
  (bind _returnvalue (`KismetMaterialLibrary.CreateDynamicMaterialInstance` "/Game/Effects/Misc/Materials/M_Dither.M_Dither"))
  (bind _output_get (set `self.MIDither` _returnvalue))
  (`PrimitiveComponent.SetMaterial` (`self.Cube`) 0 _output_get))

(event `/Game/Blueprints/Interfaces/BPI_Fadeable.Fade`
  (if (not (`self.IsFaded`))
    (set `self.IsFaded` true)
    (bind (_direction _percent) (`Timeline|FadeTL`)
      (:`Update`
        (`MaterialInstanceDynamic.SetScalarParameterValue` (`self.MIDither`) "Percent" _percent)))))

(event `/Game/Blueprints/Interfaces/BPI_Fadeable.Unfaded`
  (set `self.IsFaded` false)
  (bind (_direction _percent) (`Timeline|UnfadeTL`)
    (:`Update`
      (`MaterialInstanceDynamic.SetScalarParameterValue` (`self.MIDither`) "Percent" _percent))))

(fn `UserConstructionScript`)