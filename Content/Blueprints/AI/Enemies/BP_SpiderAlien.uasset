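; BP_SpiderAlien is an enemy that chases the player, attacks in melee and can drop a prize on death.
; BeginPlay loops AI MoveTo, while Tick halts movement to play the attack montage within range; DamagePlayer applies the hit but is called from outside this graph.
; At zero health it credits the marine's kill, notifies the game mode, then destroys itself after a delay.
; Aim events toggle a billboard marker.
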(event `self.ReceiveBeginPlay`
  (`|AIMoveTo` self (0.0 0.0 0.0) (`GameplayStatics.GetPlayerCharacter` 0) :!label _label
    (:`OnSuccess`
      _)
    (:`OnFail`
      _))
  (`KismetSystemLibrary.Delay` 0.2)
  (if (not (`self.IsDead`))
    (goto _label)))

(event `self.ReceiveTick`
  (params (DeltaSeconds :type "Float (single-precision)"))
  (bind _charactermovement (`self.CharacterMovement`))
  (if (and (`self.IsInAttackRange`) (not (`self.IsAttacking`)) (not (`self.IsDead`)))
    (`ActorComponent.Deactivate` _charactermovement)
    (`|PlayMontage` (`self.Mesh`) "/Game/Characters/Enemy_Great_Spider/Animations/AlienAttack_AM.AlienAttack_AM"
      (:`OnCompleted`
        (`ActorComponent.Activate` _charactermovement false)))))

(event `self.ReceiveAnyDamage`
  (params (Damage :type "Float (single-precision)") (DamageType :type "DamageType Object Reference") (InstigatedBy :type "Controller Object Reference") (DamageCauser :type "Actor Object Reference"))
  (bind _charactermovement (`self.CharacterMovement`))
  (if (not (`self.IsDead`))
    (bind _output_get (set `self.CurrentHealth` (`KismetMathLibrary.FClamp` (- (`self.CurrentHealth`) Damage) 0.0 100.0)))
    (if (== _output_get 0.0)
      (set `self.IsDead` true)
      (bind _asbp_marine (cast `/Game/Blueprints/Pawns/BP_Marine` (`GameplayStatics.GetPlayerCharacter` 0)))
      (`/Game/Blueprints/Pawns/BP_Marine.IncreaseKills` _asbp_marine)
      (bind _asmars_marine_game_mode (cast `/Game/Core/GameModes/MarsMarine_GameMode` (`GameplayStatics.GetGameMode`)))
      (`/Game/Core/GameModes/MarsMarine_GameMode.AlienDied` _asmars_marine_game_mode self)
      (`self.SetActorEnableCollision` false)
      (`MovementComponent.StopMovementImmediately` _charactermovement)
      (`ActorComponent.Deactivate` _charactermovement)
      (`KismetSystemLibrary.Delay` 2.0)
      (`self.SetPrize`)
      (`self.K2_DestroyActor`))))

(event `/Game/Blueprints/Interfaces/BPI_Attackable.IsOnAim`
  (if (`SceneComponent.bHiddenInGame` (`self.Billboard`))
    (`SceneComponent.SetHiddenInGame` (`self.Billboard`) false false)))

(event `/Game/Blueprints/Interfaces/BPI_Attackable.OutOfAim`
  (`SceneComponent.SetHiddenInGame` (`self.Billboard`) true false))

(fn `DamagePlayer`
  (`GameplayStatics.ApplyDamage` (`GameplayStatics.GetPlayerCharacter` 0) (`self.DamagePerHit`)))

(fn `IsAttacking`
  (returns (ReturnValue :type Boolean))
  (return (`AnimInstance.Montage_IsPlaying` (`SkeletalMeshComponent.GetAnimInstance` (`self.Mesh`)) "/Game/Characters/Enemy_Great_Spider/Animations/AlienAttack_AM.AlienAttack_AM")))

(fn `IsInAttackRange`
  (returns (ReturnValue :type Boolean))
  (return (< (`self.GetDistanceTo` (`GameplayStatics.GetPlayerCharacter` 0)) (`self.AttackRange`))))

(fn `SetPrize`
  (bind _spawnprizeclasses (`self.SpawnPrizeClasses`))
  (if (<= (`KismetMathLibrary.RandomFloat`) (`self.PrizeChance`))
    (if (> (`KismetArrayLibrary.Array_Length` _spawnprizeclasses) 0)
      (`|SpawnActorFromClass` (`KismetArrayLibrary.Array_Random` _spawnprizeclasses) (`KismetMathLibrary.MakeTransform` (`SceneComponent.K2_GetComponentLocation` (`self.Mesh`))) "AlwaysSpawn" "OverrideRootScale" null null))))

(fn `UserConstructionScript`)