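; Projectile actor from a shooting VFX pack that spawns an impact actor where it hits.
; On begin play, its sphere collider ignores the instigator while moving, so the projectile does not collide with its shooter.
; On a component hit, it disables sphere collision, spawns ImpactActor at the hit location with default rotation and scale, then destroys itself.
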(event `self.Sphere1.OnComponentHit`
  (params (HitComponent :type "PrimitiveComponent Object Reference") (OtherActor :type "Actor Object Reference") (OtherComp :type "PrimitiveComponent Object Reference") (NormalImpulse :type "Vector Structure") (Hit :type "HitResult Structure (by ref)"))
  (`PrimitiveComponent.SetCollisionEnabled` (`self.Sphere1`) "NoCollision")
  (`|SpawnActorFromClass` (`self.ImpactActor`) (`KismetMathLibrary.MakeTransform` (`.Location` (`GameplayStatics.BreakHitResult` Hit))) "Undefined" "OverrideRootScale" null null)
  (`self.K2_DestroyActor`))

(event `self.ReceiveBeginPlay`
  (`PrimitiveComponent.IgnoreActorWhenMoving` (`self.Sphere1`) (`self.GetInstigator`) true))

(fn `UserConstructionScript`)